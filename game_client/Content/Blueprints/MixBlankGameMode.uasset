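; Game mode for a Mixer interactivity sample, passing click messages between the game client and remote participants and showing them in a UI widget.
; Local clicks are broadcast to everyone; participant clicks are echoed to their sender.
; Global and per-participant click counts update the widget and are pushed back to Mixer, using a locally tracked participant list.
; Joins are faked from participant events because the plugin never broadcasts join or leave.
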(event Custom|GameClientClick
  (params (location :type Vector%202D%20Structure))
  (bind _returnvalue (Utilities|String|ToString(Vector2d) location))
  (bind _returnvalue_2 (Utilities|String|Append "Game Client Clicked at: " _returnvalue))
  ;[1 1 1] Broadcast a message to all participants
  (CallFunction|UpdateNumGlobalClicks)
  (Rendering|Components|TextRender|SetText (Variables|/Game/Blueprints/UIWidget.UIWidget_C|GetLocalGameClientMessage (Variables|Default|GetUIWidgetRef)) (Utilities|Text|ToText(String) _returnvalue_2)) ; Show local message in the game client
  ;;[1 1 1] Broadcast message to all PEs
  (Class|MixerGameClient|SendBroadcastEvent "client_click" 0.0 0.0 _returnvalue_2) ; This is a static function of MixerGameClient
)

(event Custom|OnParticipantEventSclick
  (params (ParticipantID :type Integer) (ParticipantName :type String) (X :type Float%20%28single-precision%29) (Y :type Float%20%28single-precision%29))
  (bind _returnvalue (Math|Vector2D|MakeVector2D X Y))
  (bind _returnvalue_2 (Utilities|String|ToString(Vector2d) _returnvalue))
  (bind _returnvalue_3 (Utilities|String|Append "Participant " ParticipantName " Clicked at: " _returnvalue_2))
  ;[1 1 1] Recive a message from a participant
  ;;[1 1 1] Show message received from PE
  (CallFunction|UpdateParticipantClicks ParticipantID)
  (Rendering|Components|TextRender|SetText (Variables|/Game/Blueprints/UIWidget.UIWidget_C|GetGameClientMessageFromPE (Variables|Default|GetUIWidgetRef)) (Utilities|Text|ToText(String) _returnvalue_3)) ; Show a local message in the game client
  ;;[1 1 1] Send a message to a specific participant - we'll send to the participant that just sent us a message
  (Class|MixerGameClient|SendParticipantEvent ParticipantID "pos_pong" 0.0 0.0 _returnvalue_3) ; This is a static function of MixerGameClient
)

(event Custom|OnParticipantJoin
  (params (ParticipantID :type Integer))
  (bind _returnvalue (Utilities|String|ToString(Integer) ParticipantID))
  ;[1 1 1] Adding a participant to the local list if not already tracked and messaging on player join - See the comment on joined and left events above
  (bind _found (CallFunction|FindParticipant ParticipantID))
  (if _found
    (Rendering|Components|TextRender|SetText (Variables|/Game/Blueprints/UIWidget.UIWidget_C|GetgenericMessage (Variables|Default|GetUIWidgetRef)) (Utilities|Text|ToText(String) (Utilities|String|Append "Participant ID " _returnvalue " Joined again (fake join based on click unless the plugin is changed)"))) ; Show local message in the game client
    (else
      (Utilities|Array|Add (Variables|Default|GetParticipantList) (Utilities|Struct|MakeBPParticipantData ParticipantID))
      (Rendering|Components|TextRender|SetText (Variables|/Game/Blueprints/UIWidget.UIWidget_C|GetgenericMessage (Variables|Default|GetUIWidgetRef)) (Utilities|Text|ToText(String) (Utilities|String|Append "Participant ID " _returnvalue " Joined and was added to local array (fake join based on click unless the plugin is changed)"))) ; Show local message in the game client
    )))

(event Custom|OnParticipantEventButtonclick
  (params (ParticipantID :type Integer) (ParticipantName :type String))
  ;[1 1 1] Recive a message from a participant
  ;;[1 1 1] Show message received from PE
  (Rendering|Components|TextRender|SetText (Variables|/Game/Blueprints/UIWidget.UIWidget_C|GetgenericMessage (Variables|Default|GetUIWidgetRef)) (Utilities|Text|ToText(String) (Utilities|String|Append "Hello " ParticipantName "! Your participant ID is: " (Utilities|String|ToString(Integer) ParticipantID)))) ; Show local message in the game client
)

(event Custom|OnParticipantLeave
  (params (ParticipantID :type Integer))
  ;[1 1 1] Display messaging when a player leaves - See the comment on joined and left events
  (Rendering|Components|TextRender|SetText (Variables|/Game/Blueprints/UIWidget.UIWidget_C|GetgenericMessage (Variables|Default|GetUIWidgetRef)) (Utilities|Text|ToText(String) (Utilities|String|Append "Participant ID " (Utilities|String|ToString(Integer) ParticipantID) " Left"))) ; Show local message in the game client
)

(event Custom|UpdateNumGlobalClicks
  ;[1 1 1] Send a control update
  (bind _result (Math|Integer|IncrementInt (Variables|Default|GetNumGlobalClicks))
    (:%20%20
      (Rendering|Components|TextRender|SetText (Variables|/Game/Blueprints/UIWidget.UIWidget_C|GetNumGlobalClicks (Variables|Default|GetUIWidgetRef)) (Utilities|Text|ToText(Integer) _result)) ; Show local message in the game client
      ;;[1 1 1] update control with new global value
      (Class|MixerGameClient|UpdateControlState _result))))

(event Custom|UpdateParticipantClicks
  (params (ParticipantId :type Integer))
  ;[1 1 1] Send a participant update
  (CallFunction|UpdateNumGlobalClicks) ; update the global value
  (bind (_found _participantstruct _index) (CallFunction|FindParticipant ParticipantId))
  (if _found
    (Utilities|Struct|SetmembersinBPParticipantData (Utilities|Array|Get(acopy) (Variables|Default|GetParticipantList) _index) (+ (.NumClicks (Utilities|Struct|BreakBPParticipantData _participantstruct)) 1))
    (Rendering|Components|TextRender|SetText (Variables|/Game/Blueprints/UIWidget.UIWidget_C|GetNumParticipantClicks (Variables|Default|GetUIWidgetRef)) (Utilities|Text|ToText(String) (Utilities|String|Append (Utilities|String|ToString(Integer) (+ (.NumClicks (Utilities|Struct|BreakBPParticipantData _participantstruct)) 1)) " total clicks from " (.Name (Class|MixerInteractivityBlueprintLibrary|GetRemoteParticipantInfo (.ParticipantID (Utilities|Struct|BreakBPParticipantData _participantstruct))))))) ; Show local message in the game client
    ;;[1 1 1] update participant with the new value
    (Class|MixerGameClient|SendParticipantUpdate (.ParticipantID (Utilities|Struct|BreakBPParticipantData _participantstruct)) (+ (.NumClicks (Utilities|Struct|BreakBPParticipantData _participantstruct)) 1))))

(event EventBeginPlay
  ;[1 1 1] Creating the UI we use to display messages
  (bind _returnvalue (UserInterface|CreateWidget "/Game/Blueprints/UIWidget.UIWidget_C" (Game|GetPlayerController 0)))
  (bind _output_get (Variables|Default|SetUIWidgetRef _returnvalue))
  (UserInterface|Viewport|AddtoViewport _output_get 0))

(fn ConstructionScript)

(fn FindParticipant
  (params (ParticipantID :type Integer))
  (if (!= ParticipantID -1) ; -1 is  never valid, it's used for object that have no participant ID
    (for (_array_element _array_index) (Variables|Default|GetParticipantList)
      (if (== (.ParticipantID (Utilities|Struct|BreakBPParticipantData _array_element)) ParticipantID)
        (return true _array_element _array_index)))
    (return false "" 0)
    (else
      (return false "" 0))))